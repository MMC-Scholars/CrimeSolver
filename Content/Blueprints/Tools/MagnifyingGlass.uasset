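; Magnifying glass tool that lets the player discover magnifier-type Evidence actors while it is held.
; Each Tick while InHand, Magnify sphere-traces through the glass along its forward axis, both in front and behind, to identify matching evidence.
; Unfound evidence triggers OnEvidenceFound only if DesktopPawnBP's FindEvidence also reports that actor, confirming the player is looking at it.
; A failed pawn cast quits the game.
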(event `self.ReceiveBeginPlay`
  (`parent.ReceiveBeginPlay`)
  (`self.SetActorTickEnabled` true))

(event `self.ReceiveTick`
  (params (DeltaSeconds :type "Float (single-precision)"))
  (`parent.ReceiveTick` DeltaSeconds)
  (if (`self.bInHand`)
    (bind (_evidencehit _evidenceidentified) (`self.Magnify`))
    ;[1 1 1] Checks if magnified object is evidence of type magnified and has not been found
    (if _evidenceidentified
      (bind (_evidenceref _isevidencetype) (`/Game/Blueprints/functions.IsEvidenceType` _evidencehit "NewEnumerator0"))
      (if (and _isevidencetype (not (`/Game/Blueprints/Evidence/Evidence.bEvidenceFound` _evidencehit)))
        (bind _asdesktop_pawn_bp (cast `/Game/Blueprints/DesktopPawn/DesktopPawnBP` (`GameplayStatics.GetPlayerPawn` 0))
          (:`then`
            (bind (_evidencehit_2 _evidencefound) (`/Game/Blueprints/DesktopPawn/DesktopPawnBP.Find Evidence` _asdesktop_pawn_bp))
            ;[1 1 1] Verifies if player is looking for/at the same evidence/object
            (if _evidencefound
              (for _array_element _evidencehit_2
                (bind _returnvalue (== _evidencehit _array_element))
                (if _returnvalue
                  (break)))
              (if _returnvalue
                (`/Game/Blueprints/Evidence/Evidence.On Evidence Found` _evidencehit))))
          (:`CastFailed`
            (`KismetSystemLibrary.QuitGame` null "Quit")))))
    (else
      (`KismetSystemLibrary.PrintString` "not"))))

(fn `Magnify`
  (returns (EvidenceHit :type "/Game/Blueprints/Evidence/Evidence Object Reference") (EvidenceIdentified :type Boolean))
  (locals (aObjectTypes :type "Array of EObjectTypeQuery Enum"))
  (bind _returnvalue (`self.K2_GetActorLocation`))
  (bind _returnvalue_2 (`KismetMathLibrary.GetForwardVector` (`self.K2_GetActorRotation`)))
  ;[1 1 1] Sphere tracing extended 0.5 meters on either side of the magnifying glass
  (bind (_outhit _returnvalue_3) (`KismetSystemLibrary.SphereTraceSingleForObjects` (+ _returnvalue (* _returnvalue_2 75.0)) (+ _returnvalue (* _returnvalue_2 -75.0)) 5.0 (`local.aObjectTypes`)))
  ;[1 1 1] Is identifiable evidence? (using magnifying glass)
  (if _returnvalue_3
    (bind _asevidence (cast `/Game/Blueprints/Evidence/Evidence` (`.HitActor` (`GameplayStatics.BreakHitResult` _outhit))))
    (bind (_evidenceref _isevidencetype) (`/Game/Blueprints/functions.IsEvidenceType` _asevidence "NewEnumerator0"))
    (return _evidenceref _isevidencetype)))

(fn `UserConstructionScript`
  (`parent.UserConstructionScript`)
  (set `self.tAimTransform` (`KismetMathLibrary.MakeTransform` (20.0 0.0 0.0))))