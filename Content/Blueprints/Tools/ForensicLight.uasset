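; Forensic light tool that toggles a spotlight and is built to reveal evidence.
; While lit and held, Tick runs Reveal, which line-traces along the beam with debug drawing.
; The hit branch, which moves RevealSphere and checks Evidence type, is gated by a constant false, so it never runs.
; The construction script writes RevealSphere's location to a Material Parameter Collection when the spotlight is visible, with no runtime update.
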(event `self.ReceiveBeginPlay`)

(event `self.ReceiveTick`
  (params (DeltaSeconds :type "Float (single-precision)"))
  (if (and (`self.bIsLightOn`) (`self.bInHand`))
    (`self.Reveal`)))

(event `self.Use Tool`
  (if (`self.bIsLightOn`)
    (set `self.bIsLightOn` false)
    (`self.TurnOff`)
    (else
      (set `self.bIsLightOn` true)
      (`self.TurnOn`))))

(fn `Reveal`
  (bind _spotlight (`self.SpotLight`))
  (bind _returnvalue (`SceneComponent.K2_GetComponentLocation` _spotlight))
  (bind (_outhit _returnvalue_2) (`KismetSystemLibrary.LineTraceSingleForObjects` :`Start` _returnvalue :`End` (+ _returnvalue (* (`SceneComponent.GetForwardVector` _spotlight) (`self.RevealDistance`))) :`ObjectTypes` (`|MakeArray` "ObjectTypeQuery1" "ObjectTypeQuery2" "ObjectTypeQuery4" :!type "EObjectTypeQuery Enum") :`DrawDebugType` "ForDuration"))
  (if (and false _returnvalue_2)
    (bind (_bblockinghit _binitialoverlap _time _distance _location _impactpoint _normal _impactnormal _physmat _hitactor) (`GameplayStatics.BreakHitResult` _outhit))
    (`SceneComponent.K2_SetWorldLocation` (`self.RevealSphere`) _location false false)
    (bind _asevidence (cast `/Game/Blueprints/Evidence/Evidence` _hitactor))
    (`/Game/Blueprints/functions.IsEvidenceType` _asevidence "NewEnumerator1")))

(fn `TurnOff`
  (`SceneComponent.SetVisibility` (`self.SpotLight`) false false))

(fn `TurnOn`
  (`SceneComponent.SetVisibility` (`self.SpotLight`) true false))

(fn `UserConstructionScript`
  (if (`SceneComponent.IsVisible` (`self.SpotLight`))
    (`KismetMaterialLibrary.SetVectorParameterValue` "/Game/Materials/flashlight/Collection.Collection" "Location" (`KismetMathLibrary.Conv_VectorToLinearColor` (`SceneComponent.K2_GetComponentLocation` (`self.RevealSphere`))))))