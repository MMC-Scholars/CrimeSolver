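; Handheld camera tool that photographs evidence while held and aimed, with selection toggling the scene capture's capture-on-movement.
; Use traces for evidence, confirms unfound evidence with a player trace and marks it found.
; It exports the render target as an HDR file to the Billboard content folder, also when the first trace finds nothing.
; OnCapture re-imports the file as a texture and stores it in CapturedEvidence by object name.
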(event `self.ReceiveTick`
  (params (DeltaSeconds :type "Float (single-precision)"))
  (`parent.ReceiveTick` DeltaSeconds))

(event `self.On Select`
  (`self.Select/Deselect Camera` true))

(event `self.On Deselect`
  (`self.Select/Deselect Camera` false))

(event `self.Use Tool`
  (bind _returnvalue (`KismetStringLibrary.Concat_StrStr` (`KismetSystemLibrary.GetProjectContentDirectory`) "Blueprints/Billboard/"))
  (if (and (`self.bIsInHand`) (`self.bIsAimingTool`))
    (bind (_asevidence _evidencefound_) (`/Game/Blueprints/functions.TraceForEvidence` self "NewEnumerator5" 100.0 7.5))
    (if _evidencefound_
      (if (not (`/Game/Blueprints/Evidence/Evidence.bEvidenceFound` _asevidence))
        (bind _evidencefound__2 (`/Game/Blueprints/functions.TraceFromPlayer` _asevidence))
        (if _evidencefound__2
          (`/Game/Blueprints/Evidence/Evidence.On Evidence Found` _asevidence)
          (bind _returnvalue_2 (`KismetStringLibrary.Concat_StrStr` (`KismetSystemLibrary.GetDisplayName` _asevidence) ".hdr"))
          (set `self.LastCapture` _returnvalue_2)
          (`KismetRenderingLibrary.ExportRenderTarget` (`SceneCaptureComponent2D.TextureTarget` (`self.cameraCapture`)) _returnvalue _returnvalue_2 :!label _label)
          (`self.OnCapture` _returnvalue (`KismetSystemLibrary.GetObjectName` _asevidence))))
      (else
        (goto _label)))))

(event `OnCapture`
  (params (FilePath :type String) (ObjectName :type String))
  (bind _returnvalue (`KismetStringLibrary.Concat_StrStr` ObjectName ".hdr"))
  (bind _capturedevidence (`self.CapturedEvidence`))
  (if true
    (bind _returnvalue_2 (`KismetRenderingLibrary.ImportFileAsTexture2D` (`KismetStringLibrary.Concat_StrStr` FilePath _returnvalue)))
    (message `AssetTools.RenameAssets` _returnvalue_2 (`|MakeArray` (make `AssetRenameData` _returnvalue_2 "Content/Blueprints/Billboard" _returnvalue)))
    (`BlueprintMapLibrary.Map_Add` _capturedevidence ObjectName _returnvalue_2)
    (`KismetSystemLibrary.PrintString` (`KismetSystemLibrary.GetDisplayName` (`BlueprintMapLibrary.Map_Find` _capturedevidence ObjectName)))))

(fn `Select/Deselect Camera`
  (params (`IsBeingSelected?` :type Boolean))
  (bind _isbeingselectedreturn (`/Game/Blueprints/functions.Tool Selected/Deselected` `IsBeingSelected?` self))
  (set `SceneCaptureComponent.bCaptureOnMovement` _isbeingselectedreturn (`self.cameraCapture`)))

(fn `UserConstructionScript`
  (`parent.UserConstructionScript`)
  (set `self.tAimTransform` (`KismetMathLibrary.MakeTransform` (15.0 0.0 0.0) (struct) (2.0 2.0 2.0))))