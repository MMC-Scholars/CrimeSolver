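; Game mode Blueprint for a detective-style game where evidence is collected and a suspect is accused.
; OnEvidenceCollect counts evidence, enabling CanAccuse with a message once the count equals EvidenceNeeded.
; When CanAccuse is set, OnAccuse prints a win or loss from the suspect's IsGuilty flag, then quits after a delay.
; Tick drives a looping MultiGate that repeatedly increments TraceCounter and resets it every tenth frame.
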(event `self.ReceiveBeginPlay`)

(event `self.ReceiveTick`
  (params (DeltaSeconds :type "Float (single-precision)"))
  (`|MultiGate` false true
    (:`Out 0`
      (`/Engine/EditorBlueprintResources/StandardMacros.IncrementInt` (`self.TraceCounter`) :!label _label))
    (:`Out 1`
      (goto _label))
    (:`Out 2`
      (goto _label))
    (:`Out 3`
      (goto _label))
    (:`Out 4`
      (goto _label))
    (:`Out 5`
      (goto _label))
    (:`Out 6`
      (goto _label))
    (:`Out 7`
      (goto _label))
    (:`Out 8`
      (goto _label))
    (:`Out 9`
      (set `self.TraceCounter` 0))))

(event `OnEvidenceCollect`
  (bind _result (`/Engine/EditorBlueprintResources/StandardMacros.IncrementInt` (`self.EvidenceCount`))
    (:`  `
      (bind _returnvalue (== _result (`self.EvidenceNeeded`)))
      (if _returnvalue
        ;[1 1 1] CanAccuse is currently set to true to test OnAccuse event
        (set `self.CanAccuse` _returnvalue)
        (`KismetSystemLibrary.PrintString` "You collected all the evidence you need to make a decision.")
        (else
          (`KismetSystemLibrary.PrintString` "You collected some evidence!"))))))

(event `OnAccuse`
  (params (Suspect :type "/Game/Blueprints/SuspectBP Object Reference"))
  (if (`self.CanAccuse`)
    (if (`/Game/Blueprints/SuspectBP.IsGuilty` Suspect)
      (`KismetSystemLibrary.PrintString` "You Win!")
      (`KismetSystemLibrary.Delay` 5.0)
      (`KismetSystemLibrary.QuitGame` null "Quit")
      (else
        (`KismetSystemLibrary.PrintString` "You Picked Wrong. You are dumb.")
        (`KismetSystemLibrary.Delay` 5.0)
        (`KismetSystemLibrary.QuitGame` null "Quit")))))

(fn `UserConstructionScript`)