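; Base Blueprint for a holdable item or tool that the desktop pawn picks up through interaction.
; Select and deselect events report the item's selection state through ItemSelectedDeselected, and interaction calls PickUpItem on the interacting DesktopPawnBP.
; UseTool is an empty stub, and a usability check requires the item to be in hand, plus aimed when CanOnlyUseWhenAiming is set.
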(event `On Select`
  (`/Game/Blueprints/functions.ItemSelectedDeselected` true self))

(event `On Deselect`
  (`/Game/Blueprints/functions.ItemSelectedDeselected` false self))

(event `Use Tool`
  (if true
    _))

(event `/Game/Blueprints/InteractionBPI.InteractWithObject`
  (params (Interacter :type "Pawn Object Reference"))
  (bind _asdesktop_pawn_bp (cast `/Game/Blueprints/DesktopPawn/DesktopPawnBP` Interacter))
  (`/Game/Blueprints/DesktopPawn/DesktopPawnBP.Pick Up Item` _asdesktop_pawn_bp self))

(fn `CanUseItemInHand?`
  (params (EquippedItem :type "/Game/Blueprints/Items/Item Object Reference"))
  (returns (`CanUseTool?` :type Boolean))
  (bind _bisinhand (`self.bIsInHand`))
  (return (select `bool` (`self.bCanOnlyUseWhenAiming`) :`false` _bisinhand :`true` (and _bisinhand (`self.bIsAimingItem`)))))

(fn `UserConstructionScript`
  (set `self.bIsAimingItem` false))