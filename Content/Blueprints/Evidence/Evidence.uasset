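; Evidence actor that can be marked as found, notifying the game mode of its collection.
; Construction clears the found flag and custom depth on its static mesh.
; OnEvidenceFound enables custom depth to highlight the mesh, sets the flag and calls OnEvidenceCollect on GameModeBP, quitting the game if that cast fails.
; The EvidenceFound function duplicates this logic, and neither guards against repeat calls.
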(event `self.ReceiveTick`
  (params (DeltaSeconds :type "Float (single-precision)")))

(event `On Evidence Found`
  (`PrimitiveComponent.SetRenderCustomDepth` (`self.StaticMesh`) true) ; Highlight Evidence
  (set `self.bEvidenceFound` true)
  (bind _asgame_mode_bp (cast `/Game/Blueprints/GameModeBP` (`GameplayStatics.GetGameMode`))
    (:`then`
      (`/Game/Blueprints/GameModeBP.OnEvidenceCollect` _asgame_mode_bp))
    (:`CastFailed`
      (`KismetSystemLibrary.QuitGame` null "Quit") ; Should never fire
    )))

(fn `EvidenceFound`
  (`PrimitiveComponent.SetRenderCustomDepth` (`self.StaticMesh`) true)
  (set `self.bEvidenceFound` true)
  (bind _asgame_mode_bp (cast `/Game/Blueprints/GameModeBP` (`GameplayStatics.GetGameMode`))
    (:`then`
      (`/Game/Blueprints/GameModeBP.OnEvidenceCollect` _asgame_mode_bp))
    (:`CastFailed`
      (`KismetSystemLibrary.QuitGame` null "Quit") ; Should never fire
    )))

(fn `UserConstructionScript`
  (set `self.bEvidenceFound` false)
  (`PrimitiveComponent.SetRenderCustomDepth` (`self.StaticMesh`) false))