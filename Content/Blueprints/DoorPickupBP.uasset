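; Grabbable door actor, likely for VR, that tracks a holding controller and ticks from pickup until drop.
; Each tick computes a clamped signed angle between the starting door direction and the unnormalized flattened pivot-to-hand vector, then sets Pivot rotation from GetRotation.
; The rotation helpers' interpolation nodes are unconnected, so the clamped angle never drives the pivot.
; An alternative min/max limit branch never runs.
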(event `self.ReceiveBeginPlay`
  (set `self.DoorDirection` (`SceneComponent.GetRightVector` (`self.Pivot`))))

(event `OnPickup_1`
  (params (controller :type "BaseController Object Reference"))
  (set `self.Controller` controller)
  (`self.SetActorTickEnabled` true))

(event `OnDrop_1`
  (params (controller :type "BaseController Object Reference"))
  (`self.SetActorTickEnabled` false)
  (set `self.Controller` null))

(event `self.ReceiveTick`
  (params (DeltaSeconds :type "Float (single-precision)"))
  (set `self.CurrentAngle` (`KismetMathLibrary.ClampAngle` (`self.GetDoorAngle`) (`self.MinAngle`) (`self.MaxAngle`)))
  (`SceneComponent.K2_SetWorldRotation` (`self.Pivot`) (`KismetMathLibrary.RInterpTo_Constant` (`SceneComponent.K2_GetComponentRotation` (`self.Pivot`)) (`self.GetDoorRotation` (`self.DoorDirection`) true) (`GameplayStatics.GetWorldDeltaSeconds`)) false false))

(fn `GetDoorAngle`
  (returns (`Return Value` :type "Float (double-precision)"))
  (return (* (`KismetMathLibrary.DegAcos` (`KismetMathLibrary.Dot_VectorVector` (`self.GetHandDoorDirection`) (`self.DoorDirection`))) (`KismetMathLibrary.SelectFloat` -1.0 1.0 (< (.z (`KismetMathLibrary.Cross_VectorVector` (`self.GetHandDoorDirection`) (`self.DoorDirection`))) 0.0)))))

(fn `GetDoorRotation`
  (params (`Optional Direction` :type "Vector Structure") (`Use Direction` :type Boolean))
  (returns (`Return Value` :type "Rotator Structure"))
  (return (`KismetMathLibrary.MakeRotFromYZ` (`KismetMathLibrary.SelectVector` `Optional Direction` (`self.GetHandDoorDirection`) `Use Direction`) (`SceneComponent.GetUpVector` (`self.Door`)))))

(fn `GetHandDoorDirection`
  (returns (`Return Value` :type "Vector Structure"))
  (return (`KismetMathLibrary.MakeVector` (.x (- (`self.K2_GetActorLocation` (`self.Controller`)) (`SceneComponent.K2_GetComponentLocation` (`self.Pivot`)))) (.y (- (`self.K2_GetActorLocation` (`self.Controller`)) (`SceneComponent.K2_GetComponentLocation` (`self.Pivot`)))))))

(fn `UserConstructionScript`)