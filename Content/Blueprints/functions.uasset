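; Function library for an evidence-finding game, providing shared checks for tools, player view and evidence detection.
; Helpers toggle a tool's in-hand visibility, test facing by camera dot product, and confirm evidence through the desktop pawn's FindEvidence.
; TraceForEvidence runs a forward, optionally two-sided, sphere trace ignoring inventory items, with debug drawing and printing.
; Its hit feeds IsEvidenceType, which as written always returns false.
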(fn `IsActorFacingPlayer`
  (params (Actor :type "Actor Object Reference"))
  (returns (`IsActorFacingPlayer?` :type Boolean))
  (bind _asdesktop_pawn_bp (cast `/Game/Blueprints/DesktopPawn/DesktopPawnBP` (`GameplayStatics.GetPlayerPawn` Actor)))
  (bind _returnvalue (`SceneComponent.GetForwardVector` (`/Game/Blueprints/DesktopPawn/DesktopPawnBP.Camera` _asdesktop_pawn_bp)))
  (return (< (/ (`KismetMathLibrary.Dot_VectorVector` (`Actor.GetActorForwardVector` Actor) _returnvalue) (`KismetMathLibrary.VSize` _returnvalue)) 0.0)))

(fn `IsEvidenceType`
  (params (Evidence :type "/Game/Blueprints/Interactables/Items/Evidence/Evidence Object Reference") (`Evidence Type` :type "/Game/Blueprints/Interactables/Items/Evidence/EEvidenceTypes Enum" :default "NewEnumerator0"))
  (returns (EvidenceRef :type "/Game/Blueprints/Interactables/Items/Evidence/Evidence Object Reference") (IsEvidenceType :type Boolean))
  (return Evidence false))

(fn `ItemSelectedDeselected`
  (params (`IsBeingSelected?` :type Boolean) (Tool :type "/Game/Blueprints/Interactables/Items/Item Object Reference"))
  (returns (IsBeingSelectedReturn :type Boolean))
  (bind _output_get (set `/Game/Blueprints/Interactables/Items/Item.bIsInHand` `IsBeingSelected?` Tool))
  (`Actor.SetActorHiddenInGame` Tool (not _output_get))
  (return _output_get))

(fn `TraceForEvidence`
  (params (EvidenceType :type "/Game/Blueprints/Interactables/Items/Evidence/EEvidenceTypes Enum" :default "NewEnumerator0") (TracingActor :type "Actor Object Reference") (TraceRadius :type "Float (double-precision)") (TraceDistance :type "Float (double-precision)" :default 75.0) (`TraceBothSides?` :type Boolean))
  (returns (AsEvidence :type "/Game/Blueprints/Interactables/Items/Evidence/Evidence Object Reference") (`EvidenceFound?` :type Boolean))
  (locals (aObjectTypes :type "Array of EObjectTypeQuery Enum"))
  ;[1 1 1] Sphere tracing extended X distance from the specified actor in the x-axis
  (bind _asdesktop_pawn_bp (cast `/Game/Blueprints/DesktopPawn/DesktopPawnBP` (`GameplayStatics.GetPlayerPawn` TracingActor)))
  (bind (_hitactor _actorhit_) (`self.TraceFromActor` TracingActor TraceRadius TraceDistance `TraceBothSides?` (`local.aObjectTypes`) (`/Game/Blueprints/DesktopPawn/Inventory.InventoryItems` (`/Game/Blueprints/DesktopPawn/DesktopPawnBP.Inventory` _asdesktop_pawn_bp)) _asdesktop_pawn_bp))
  (`KismetSystemLibrary.PrintString` _hitactor (`KismetSystemLibrary.GetDisplayName` _hitactor))
  ;[1 1 1] Is identifiable evidence?
  (if _actorhit_
    (bind _asevidence (cast `/Game/Blueprints/Interactables/Items/Evidence/Evidence` _hitactor))
    (bind (_evidenceref _isevidencetype) (`self.IsEvidenceType` _asevidence EvidenceType _asevidence))
    (return _evidenceref _isevidencetype)))

(fn `TraceFromActor`
  (params (TracingActor :type "Actor Object Reference") (TraceRadius :type "Float (double-precision)") (TraceDistance :type "Float (double-precision)") (TraceBothSides :type Boolean) (ObjectTypes :type "Array of EObjectTypeQuery Enum") (ActorsToIgnore :type "Array of /Game/Blueprints/Interactables/Items/Item Object Reference"))
  (returns (HitActor :type "Actor Object Reference") (`ActorHit?` :type Boolean))
  (bind _returnvalue (`Actor.K2_GetActorLocation` TracingActor))
  (bind _returnvalue_2 (`KismetMathLibrary.GetForwardVector` (`Actor.K2_GetActorRotation` TracingActor)))
  (bind (_outhit _returnvalue_3) (`KismetSystemLibrary.SphereTraceSingleForObjects` TracingActor (select `bool` TraceBothSides :`false` _returnvalue :`true` (+ _returnvalue (* _returnvalue_2 (* TraceDistance -1.0)))) (+ _returnvalue (* _returnvalue_2 TraceDistance)) TraceRadius ObjectTypes false ActorsToIgnore "ForDuration"))
  (return (`.HitActor` (`GameplayStatics.BreakHitResult` _outhit)) _returnvalue_3))

(fn `TraceFromPlayer`
  (params (IdentifiedEvidence :type "/Game/Blueprints/Interactables/Items/Evidence/Evidence Object Reference"))
  (returns (`EvidenceFound?` :type Boolean))
  (bind _asdesktop_pawn_bp (cast `/Game/Blueprints/DesktopPawn/DesktopPawnBP` (`GameplayStatics.GetPlayerPawn` IdentifiedEvidence))
    (:`then`
      (bind (_evidencehit _evidencefound) (`/Game/Blueprints/DesktopPawn/DesktopPawnBP.Find Evidence` _asdesktop_pawn_bp))
      (if _evidencefound
        (for _array_element _
          (bind _returnvalue (== IdentifiedEvidence _array_element))
          (if _returnvalue
            (break)))
        (return _returnvalue)))
    (:`CastFailed`
      (`KismetSystemLibrary.QuitGame` IdentifiedEvidence null "Quit"))))