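; An interactable in-world 3D menu that switches control from the player to a menu camera so its widget can be used with the mouse.
; Interaction possesses MenuCamera, hides the player, shows the cursor and enables UI collision on the widget, and PossessPlayer reverses this.
; On BeginPlay it checks its level-assigned camera and player references, then hands itself to MainMenuBP.
; ChangeWidget swaps the displayed screen.
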(event `self.ReceiveBeginPlay`
  (`/Engine/EditorBlueprintResources/StandardMacros.IsValid` (`self.MenuCamera`)
    (:`Is Valid`
      (`/Engine/EditorBlueprintResources/StandardMacros.IsValid` (`self.Player`)
        (:`Is Valid`
          (bind _asmain_menu_bp (cast `/Game/Blueprints/UI/Menus/MainMenuBP` (`WidgetComponent.GetUserWidgetObject` (`self.Widget`))))
          (set `/Game/Blueprints/UI/Menus/MenuBP.3DMenuRef` self _asmain_menu_bp))
        (:`Is Not Valid`
          (`Debug.LogError` "Error: Player was not given a reference from the level"))))
    (:`Is Not Valid`
      (`Debug.LogError` "Error: MenuCamera was not given a reference from the level"))))

(event `/Game/Blueprints/InteractionBPI.InteractWithObject`
  (params (Interacter :type "Pawn Object Reference") (HitLocation :type "Vector Structure") (LocationNormal :type "Vector Structure"))
  (`self.Possess Camera`))

(event `Change Widget`
  (params (Widget :type "/Game/Blueprints/UI/Menus/MenuBP Object Reference"))
  (`/Engine/EditorBlueprintResources/StandardMacros.IsValid` Widget
    (:`Is Valid`
      (`WidgetComponent.SetWidget` (`self.Widget`) Widget))
    (:`Is Not Valid`
      (`Debug.LogError` "Error: Tried to change widget with null reference"))))

(event `Possess Player`
  (bind _returnvalue (`GameplayStatics.GetPlayerController` 0))
  (bind _player (`self.Player`))
  (`Controller.Possess` _returnvalue _player)
  (`self.SetActorHiddenInGame` _player false)
  (set `PlayerController.bShowMouseCursor` false _returnvalue)
  (`WidgetBlueprintLibrary.SetInputMode_GameOnly` _returnvalue)
  (`PrimitiveComponent.SetCollisionProfileName` (`self.Widget`) "NoCollision" true))

(event `Possess Camera`
  (bind _returnvalue (`GameplayStatics.GetPlayerController` 0))
  (bind _player (`self.Player`))
  (`self.SetActorHiddenInGame` _player true)
  (`/Game/Blueprints/DesktopPawn/DesktopCharacterBP.ChangeTools` _player 0)
  (`Controller.Possess` _returnvalue (`self.MenuCamera`))
  (set `PlayerController.bShowMouseCursor` true _returnvalue)
  (`WidgetBlueprintLibrary.SetInputMode_GameAndUIEx` _returnvalue null)
  (`PrimitiveComponent.SetCollisionProfileName` (`self.Widget`) "UI" true))

(fn `UserConstructionScript`)