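; An interactable light switch that toggles a set of referenced lights.
; Each interaction flips the IsFlippedUp state, rotates the Switch component to match, and inverts the visibility of every valid entry in the Lights array.
; The construction script poses the switch from IsFlippedUp but leaves the lights untouched, so each light toggles from its own current visibility rather than following the switch position.
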(event `self.ReceiveBeginPlay`)

(event `/Game/Blueprints/InteractionBPI.InteractWithObject`
  (params (Interacter :type "Pawn Object Reference") (HitLocation :type "Vector Structure") (LocationNormal :type "Vector Structure"))
  (if (`self.isFlippedUp`)
    (set `self.isFlippedUp` false)
    (`self.FlipDown`)
    (else
      (set `self.isFlippedUp` true)
      (`self.FlipUp`)))
  (for _array_element (`self.Lights`)
    (`/Engine/EditorBlueprintResources/StandardMacros.IsValid` _array_element
      (:`Is Valid`
        (`self.ToggleLight` _array_element)))))

(fn `FlipDown`
  (`SceneComponent.K2_SetRelativeRotation` :`self` (`self.Switch`)))

(fn `FlipUp`
  (locals (LocLight :type "Object Object Reference") (FlipRotation :type "Rotator Structure" :default (struct)))
  (`SceneComponent.K2_SetRelativeRotation` (`self.Switch`) (struct :`Roll` 180.0) false false))

(fn `ToggleLight`
  (params (Light :type "Light Object Reference"))
  (locals (LocLight :type "Light Object Reference"))
  (bind _lightcomponent (`Light.LightComponent` Light))
  (`SceneComponent.SetVisibility` _lightcomponent (not (`SceneComponent.bVisible` _lightcomponent)) false))

(fn `UserConstructionScript`
  (if (`self.isFlippedUp`)
    (`self.FlipUp`)
    (else
      (`self.FlipDown`))))