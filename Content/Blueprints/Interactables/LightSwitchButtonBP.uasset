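; An interactable light switch that toggles a point light on and off.
; The InteractwithObject event flips the IsLightOn flag and calls TurnOn or TurnOff.
; Those functions set the PointLight visibility and snap the Switch component's relative rotation half a turn to match the state.
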(event `/Game/Blueprints/InteractionBPI.InteractWithObject`
  (params (Interacter :type "Pawn Object Reference") (HitLocation :type "Vector Structure") (LocationNormal :type "Vector Structure"))
  (if (`self.isLightOn`)
    (set `self.isLightOn` false)
    (`self.TurnOff`)
    (else
      (set `self.isLightOn` true)
      (`self.TurnOn`))))

(fn `TurnOff`
  (`SceneComponent.SetVisibility` (`self.PointLight`) false false)
  (`SceneComponent.K2_SetRelativeRotation` (`self.Switch`) (struct) false false))

(fn `TurnOn`
  (`SceneComponent.SetVisibility` (`self.PointLight`) true false)
  (`SceneComponent.K2_SetRelativeRotation` (`self.Switch`) (struct :`Roll` 180.0) false false))

(fn `UserConstructionScript`)