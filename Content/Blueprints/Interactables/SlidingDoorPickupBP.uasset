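; Interactable sliding door or drawer that toggles open and closed on a desktop interaction event.
; On BeginPlay it takes the local transforms of the first two spline points as its closed and open poses.
; An Open/Close macro eases the Drawer component between them with MoveComponentTo, signalling start and completion.
; Those signals drive IsOpening and IsClosing flags, which block reversing the movement until it finishes.
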(event `self.ReceiveBeginPlay`
  (set `self.StartTransform` (`SplineComponent.GetTransformAtSplinePoint` (`self.Spline`) 0 "Local" false))
  (set `self.EndTransform` (`SplineComponent.GetTransformAtSplinePoint` (`self.Spline`) 1 "Local" false)))

(event `/Game/Blueprints/InteractionBPI.InteractWithObject`
  (params (Interacter :type "Pawn Object Reference") (HitLocation :type "Vector Structure") (LocationNormal :type "Vector Structure"))
  ;[1 1 1] Desktop Interaction
  (if (`self.IsOpen`)
    (if (not (`self.IsOpening`))
      (set `self.IsOpen` false)
      (`self.Open/Close` (`self.StartTransform`) 0.5 ; Closing
        (:`First`
          (set `self.IsClosing` true))
        (:`Completed`
          (set `self.IsClosing` false))))
    (elif (not (`self.IsClosing`))
      (set `self.IsOpen` true)
      (`self.Open/Close` (`self.EndTransform`) 0.5 ; Opening
        (:`First`
          (set `self.IsOpening` true))
        (:`Completed`
          (set `self.IsOpening` false))))))

(fn `UserConstructionScript`)