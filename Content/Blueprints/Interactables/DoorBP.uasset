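; Swinging door interactable that supports both VR controllers and desktop pawns, ticking only while held or interacted with.
; In VR it sets the pivot rotation through helpers chosen by comparing the current angle to min and max limits.
; On desktop, changes in character yaw swing the pivot within yaw bounds, signed by the side the pawn faces.
; Desktop interaction stops when the knob leaves the character's reach.
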(event `self.ReceiveBeginPlay`
  (set `self.DoorDirection` (`SceneComponent.GetRightVector` (`self.Pivot`)))
  (bind _output_get (set `self.Door Rotation` (`SceneComponent.K2_GetComponentRotation` (`self.Pivot`))))
  (set `self.DoorYaw` (.yaw _output_get)))

(event `self.OnPickup`
  (params (controller :type "BaseController Object Reference"))
  ;[1 1 1] VR Interaction
  (set `self.Controller` controller)
  (`self.SetActorTickEnabled` true))

(event `self.OnDrop`
  (params (controller :type "BaseController Object Reference"))
  ;[1 1 1] VR Interaction
  (`self.SetActorTickEnabled` false)
  (set `self.Controller` null))

(event `self.InteractWithObject`
  (params (Interacter :type "Pawn Object Reference") (HitLocation :type "Vector Structure") (LocationNormal :type "Vector Structure"))
  ;[1 1 1] Desktop Interaction
  (set `self.Pawn` Interacter)
  (`self.SetActorTickEnabled` true)
  (set `self.CharacterPrevYaw` (`self.GetCharacterYaw`))
  (set `self.DoorSwingSpeed` (`self.GetDoorSwing`)))

(event `self.StopInteractWithObject`
  ;[1 1 1] Desktop Interaction
  (`self.SetActorTickEnabled` false)
  (set `self.Pawn` null))

(event `self.ReceiveTick`
  (params (DeltaSeconds :type "Float (single-precision)"))
  (bind _return_value (`self.GetCharacterYaw`))
  (bind _returnvalue (`KismetMathLibrary.ComposeRotators` (`SceneComponent.K2_GetComponentRotation` (`self.Pivot`)) (`KismetMathLibrary.MakeRotator` 0.0 0.0 (* (/ (- (`self.CharacterPrevYaw`) _return_value) DeltaSeconds) (`self.DoorSwingSpeed`)))))
  (if (`KismetSystemLibrary.IsValid` (`self.Controller`))
    (if (<= (`self.CurrentAngle`) (`self.MinAngle`))
      (`SceneComponent.K2_SetWorldRotation` (`self.Pivot`) (`KismetMathLibrary.RInterpTo_Constant` (`SceneComponent.K2_GetComponentRotation` (`self.Pivot`)) (`self.GetDoorRotation` (`self.DoorDirection`)) (`GameplayStatics.GetWorldDeltaSeconds`) 500.0) false false)
      (elif (>= (`self.CurrentAngle`) (`self.MaxAngle`))
        (`SceneComponent.K2_SetWorldRotation` (`self.Pivot`) (`KismetMathLibrary.RInterpTo_Constant` (`SceneComponent.K2_GetComponentRotation` (`self.Pivot`)) (`self.GetDoorRotation` (`KismetMathLibrary.RotateAngleAxis` (`self.DoorDirection`) (`self.MaxAngle`) (`KismetMathLibrary.NegateVector` (`SceneComponent.GetUpVector` (`self.Pivot`)))) true) (`GameplayStatics.GetWorldDeltaSeconds`)) false false)
        (else
          (`SceneComponent.K2_SetWorldRotation` (`self.Pivot`) (`KismetMathLibrary.RInterpTo_Constant` (`SceneComponent.K2_GetComponentRotation` (`self.Pivot`)) (`self.GetDoorRotation` (0.0 0.0 0.0)) (`GameplayStatics.GetWorldDeltaSeconds`)) false false))))
    (elif (`self.Is in Reach`)
      (if (`self.Rotation in Bounds` _returnvalue)
        (`SceneComponent.K2_SetWorldRotation` (`self.Pivot`) _returnvalue false false)
        (set `self.CharacterPrevYaw` _return_value))
      (else
        (`self.StopInteractWithObject`)))))

(fn `GetCharacterYaw`
  (returns (`Return Value` :type "Float (double-precision)"))
  (return (.yaw (`SceneComponent.K2_GetComponentRotation` (`Actor.RootComponent` (`self.Pawn`))))))

(fn `GetDoorAngle`
  (returns (`Return Value` :type "Float (double-precision)"))
  (return (* (`KismetMathLibrary.DegAcos` (`KismetMathLibrary.Dot_VectorVector` (`self.GetHandDoorDirection`) (`self.DoorDirection`))) (`KismetMathLibrary.SelectFloat` -1.0 1.0 (< (.z (`KismetMathLibrary.Cross_VectorVector` (`self.GetHandDoorDirection`) (`self.DoorDirection`))) 0.0)))))

(fn `GetDoorRotation`
  (params (`Optional Direction` :type "Vector Structure") (`Use Direction` :type Boolean))
  (returns (`Return Value` :type "Rotator Structure"))
  (return (`KismetMathLibrary.MakeRotFromYZ` (`KismetMathLibrary.SelectVector` `Optional Direction` (`self.GetHandDoorDirection`) `Use Direction`) (`SceneComponent.GetUpVector` (`self.Door`)))))

(fn `GetDoorSwing`
  (returns (`Return Value` :type "Float (double-precision)"))
  (if (< (`KismetMathLibrary.Dot_VectorVector` (`SceneComponent.GetForwardVector` (`self.Arrow`)) (`self.GetActorForwardVector` (`self.Pawn`))) 0.0)
    (if (> (`self.DoorSwingSpeed`) 0.0)
      (return (`self.DoorSwingSpeed`))
      (else
        (return (* (`self.DoorSwingSpeed`) -1.0))))
    (elif (< (`self.DoorSwingSpeed`) 0.0)
      (return (`self.DoorSwingSpeed`))
      (else
        (return (* (`self.DoorSwingSpeed`) -1.0))))))

(fn `GetHandDoorDirection`
  (returns (`Return Value` :type "Vector Structure"))
  (return (`KismetMathLibrary.MakeVector` (.x (- (`self.K2_GetActorLocation` (`self.Controller`)) (`SceneComponent.K2_GetComponentLocation` (`self.Pivot`)))) (.y (- (`self.K2_GetActorLocation` (`self.Controller`)) (`SceneComponent.K2_GetComponentLocation` (`self.Pivot`)))))))

(fn `Is in Reach`
  (returns (`Return Value` :type Boolean))
  (bind _asdesktop_character_bp (cast `/Game/Blueprints/DesktopPawn/DesktopCharacterBP` (`self.Pawn`)))
  (return (> (`/Game/Blueprints/DesktopPawn/DesktopCharacterBP.fInteractionDistance` _asdesktop_character_bp) (`KismetMathLibrary.VSize` (- (`SceneComponent.K2_GetComponentLocation` (`self.Knob`)) (`SceneComponent.K2_GetComponentLocation` (`Actor.RootComponent` (`self.Pawn`))))))))

(fn `Rotation in Bounds`
  (params (`New Rotation` :type "Rotator Structure (by ref)"))
  (returns (`Return Value` :type Boolean))
  (bind _yaw (.yaw `New Rotation`))
  (return (and (> _yaw (+ (`self.DoorYaw`) (`self.MinAngle`))) (< _yaw (+ (`self.DoorYaw`) (`self.MaxAngle`))))))

(fn `UserConstructionScript`)