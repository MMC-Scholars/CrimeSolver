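; Billboard actor on which the player pins the Image held in the current inventory slot by interacting with it.
; Placement clamps the hit point inside the board's Box, then nudges it along the surface normal while it overlaps other Images, layering them.
; Box overlaps track PolaroidInstants and unpin them on exit; Tick disables pickup physics on pinned Images and prints debug text.
; A failed inventory removal quits the game.
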(event `self.ReceiveTick`
  (params (DeltaSeconds :type "Float (single-precision)"))
  (bind (_outactors _returnvalue) (`KismetSystemLibrary.ComponentOverlapActors` (`self.Box`) (`self.GetTransform`) (`|MakeArray` "ObjectTypeQuery1" "ObjectTypeQuery2" "ObjectTypeQuery7" :!type "EObjectTypeQuery Enum") "/Game/Blueprints/Interactables/Items/Images/Image.Image_C"))
  (if _returnvalue
    (for _array_element _outactors
      (bind _asimage (cast `/Game/Blueprints/Interactables/Items/Images/Image` _array_element)
        (:`then`
          (if (`/Game/Blueprints/Interactables/Items/Images/Image.bIsPinned` _asimage)
            (`Pickup.SetSimulatePickupPhysics` _asimage false)
            (else
              (`KismetSystemLibrary.PrintString` "bruh" :!label _label))))
        (:`CastFailed`
          (goto _label))))
    (`KismetSystemLibrary.PrintString` (`KismetStringLibrary.Conv_IntToString` (`KismetArrayLibrary.Array_Length` _outactors)))))

(event `/Game/Blueprints/InteractionBPI.InteractWithObject`
  (params (Interacter :type "Pawn Object Reference") (HitLocation :type "Vector Structure") (LocationNormal :type "Vector Structure"))
  (bind _asdesktop_pawn_bp (cast `/Game/Blueprints/DesktopPawn/DesktopPawnBP` Interacter))
  (bind _asimage (cast `/Game/Blueprints/Interactables/Items/Images/Image` (`|GetArrayItem` (`/Game/Blueprints/DesktopPawn/Inventory.Items` (`/Game/Blueprints/DesktopPawn/DesktopPawnBP.Inventory` _asdesktop_pawn_bp)) (`/Game/Blueprints/DesktopPawn/DesktopPawnBP.iCurrentInventorySlot` _asdesktop_pawn_bp))))
  (`self.AddImageToBillboard` _asdesktop_pawn_bp _asimage HitLocation LocationNormal))

(event `self.Box.OnComponentBeginOverlap`
  (params (OverlappedComponent :type "PrimitiveComponent Object Reference") (OtherActor :type "Actor Object Reference") (OtherComp :type "PrimitiveComponent Object Reference") (OtherBodyIndex :type Integer) (bFromSweep :type Boolean) (SweepResult :type "HitResult Structure (by ref)"))
  (bind _aspolaroid_instant (cast `/Game/Blueprints/Interactables/Items/Images/PolaroidInstant` OtherActor))
  (`KismetArrayLibrary.Array_Add` (`self.aPinnedImages`) _aspolaroid_instant))

(event `self.Box.OnComponentEndOverlap`
  (params (OverlappedComponent :type "PrimitiveComponent Object Reference") (OtherActor :type "Actor Object Reference") (OtherComp :type "PrimitiveComponent Object Reference") (OtherBodyIndex :type Integer))
  (bind _aspolaroid_instant (cast `/Game/Blueprints/Interactables/Items/Images/PolaroidInstant` OtherActor))
  (`KismetArrayLibrary.Array_RemoveItem` (`self.aPinnedImages`) _aspolaroid_instant)
  (set `/Game/Blueprints/Interactables/Items/Images/Image.bIsPinned` false _aspolaroid_instant))

(fn `AddImageToBillboard`
  (params (DesktopPawnRef :type "/Game/Blueprints/DesktopPawn/DesktopPawnBP Object Reference") (Image :type "/Game/Blueprints/Interactables/Items/Images/Image Object Reference") (TracedLocation :type "Vector Structure") (TracedSurfaceNormal :type "Vector Structure"))
  (bind _imagetransform (`self.ImageOverlapPositioning` Image TracedLocation TracedSurfaceNormal DesktopPawnRef))
  (bind (_removeditem _wasitemremoved) (`/Game/Blueprints/DesktopPawn/Inventory.RemoveSlotFromInventory` (`/Game/Blueprints/DesktopPawn/DesktopPawnBP.Inventory` DesktopPawnRef) (`/Game/Blueprints/DesktopPawn/DesktopPawnBP.iCurrentInventorySlot` DesktopPawnRef)))
  (if _wasitemremoved
    (`self.K2_SetActorTransform` _removeditem _imagetransform false false)
    (set `/Game/Blueprints/Interactables/Items/Images/Image.bIsPinned` true Image)
    (set `/Game/Blueprints/Interactables/Items/Images/Image.CurrentBillboard` self Image)
    (else
      (`KismetSystemLibrary.QuitGame` null "Quit"))))

(fn `ImageOverlapPositioning`
  (params (ImageToBePinned :type "/Game/Blueprints/Interactables/Items/Images/Image Object Reference") (TraceHitLocation :type "Vector Structure") (TraceSurfaceNormal :type "Vector Structure") (Player :type "/Game/Blueprints/DesktopPawn/DesktopPawnBP Object Reference"))
  (returns (ImageTransform :type "Transform Structure"))
  (locals (vImagePosition :type "Vector Structure") (bIsOverlap :type Boolean :default true) (ObjectTypes :type "Array of EObjectTypeQuery Enum") (bCastSucceeded :type Boolean) (IgnoredActors :type "Array of Actor Object Reference") (bIsInBillboardBounds :type Boolean))
  (bind _x (.x TraceHitLocation))
  (bind _y (.y TraceHitLocation))
  (bind _z (.z TraceHitLocation))
  (bind _box (`/Game/Blueprints/Interactables/Items/Images/Image.Box` ImageToBePinned))
  (bind _box_2 (`self.Box`))
  (bind _returnvalue (`SceneComponent.K2_GetComponentLocation` _box_2))
  (bind _returnvalue_2 (`BoxComponent.GetScaledBoxExtent` _box))
  (bind _returnvalue_3 (`BoxComponent.GetScaledBoxExtent` _box_2))
  (bind (_returnvalue_x _returnvalue_y _returnvalue_z) (`KismetMathLibrary.BreakVector` (- TraceHitLocation _returnvalue_2)))
  (bind (_returnvalue_x_2 _returnvalue_y_2 _returnvalue_z_2) (`KismetMathLibrary.BreakVector` (- _returnvalue _returnvalue_3)))
  (bind _returnvalue_4 (`KismetMathLibrary.MakeTransform` (`local.vImagePosition`) (`KismetMathLibrary.MakeRotFromXZ` TraceSurfaceNormal (`self.GetActorUpVector`)) (`/Game/Blueprints/Interactables/Items/Images/Image.vPinnedImageScale` ImageToBePinned)))
  (bind (_returnvalue_x_3 _returnvalue_y_3 _returnvalue_z_3) (`KismetMathLibrary.BreakVector` (+ TraceHitLocation _returnvalue_2)))
  (bind (_returnvalue_x_4 _returnvalue_y_4 _returnvalue_z_4) (`KismetMathLibrary.BreakVector` (+ _returnvalue _returnvalue_3)))
  (bind _returnvalue_5 (> _returnvalue_x_3 _returnvalue_x_4))
  (bind _returnvalue_6 (> _returnvalue_y_3 _returnvalue_y_4))
  (bind _returnvalue_7 (> _returnvalue_z_3 _returnvalue_z_4))
  (bind _returnvalue_8 (and (not _returnvalue_7) (not (< _returnvalue_z _returnvalue_z_2))))
  (bind _output_get (set `local.IgnoredActors` (`/Game/Blueprints/DesktopPawn/Inventory.Items` (`/Game/Blueprints/DesktopPawn/DesktopPawnBP.Inventory` Player))))
  (`KismetArrayLibrary.Array_Add` _output_get Player)
  (`KismetArrayLibrary.Array_Add` _output_get self)
  ;[1 1 1] Get a position of image that is within bounds of the billboard
  (if (not (or (> (.x (`BoxComponent.BoxExtent` (`/Game/Blueprints/Interactables/Items/Images/Image.Box` ImageToBePinned))) (.x (`BoxComponent.BoxExtent` (`self.Box`)))) (> (.y (`BoxComponent.BoxExtent` (`/Game/Blueprints/Interactables/Items/Images/Image.Box` ImageToBePinned))) (.y (`BoxComponent.BoxExtent` (`self.Box`)))) (> (.z (`BoxComponent.BoxExtent` (`/Game/Blueprints/Interactables/Items/Images/Image.Box` ImageToBePinned))) (.z (`BoxComponent.BoxExtent` (`self.Box`))))))
    (set `local.vImagePosition` (`KismetMathLibrary.MakeVector` (select `bool` (and (not _returnvalue_5) (not (< _returnvalue_x _returnvalue_x_2))) :`false` (select `bool` _returnvalue_5 :`false` (- _x (- _returnvalue_x _returnvalue_x_2)) :`true` (- _x (- _returnvalue_x_3 _returnvalue_x_4))) :`true` (.x TraceHitLocation)) (select `bool` (and (not _returnvalue_6) (not (< _returnvalue_y _returnvalue_y_2))) :`false` (select `bool` _returnvalue_6 :`false` (- _y (- _returnvalue_y _returnvalue_y_2)) :`true` (- _y (- _returnvalue_y_3 _returnvalue_y_4))) :`true` (.y TraceHitLocation)) (select `bool` _returnvalue_8 :`false` (select `bool` _returnvalue_7 :`false` (- _z (- _returnvalue_z _returnvalue_z_2)) :`true` (- _z (- _returnvalue_z_3 _returnvalue_z_4))) :`true` (.z TraceHitLocation))))
    (`KismetSystemLibrary.PrintString` (`KismetStringLibrary.Conv_BoolToString` _returnvalue_8))
    (while (`local.bIsOverlap`)
      (bind (_outactors _returnvalue_9) (`KismetSystemLibrary.ComponentOverlapActors` _box _returnvalue_4 (`local.ObjectTypes`) "/Game/Blueprints/Interactables/Items/Images/Image.Image_C" (`local.IgnoredActors`)))
      (bind _output_get_2 (set `local.bIsOverlap` _returnvalue_9))
      (if _output_get_2
        (for _array_element _outactors
          (bind _asbillboard (cast `/Game/Blueprints/Boards/BIllboard` _array_element))
          (`KismetArrayLibrary.Array_Add` (`local.IgnoredActors`) _asbillboard)
          (set `local.bCastSucceeded` true))
        (if (`local.bCastSucceeded`)
          (set `local.bCastSucceeded` false)
          (else
            (set `local.vImagePosition` (+ (`local.vImagePosition`) TraceSurfaceNormal))))))
    (return _returnvalue_4)))

(fn `UserConstructionScript`)