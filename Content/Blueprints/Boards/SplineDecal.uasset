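; SplineDecal is an actor that records points on a spline and stamps marker decals at them, apparently for drawing on boards.
; AddDecalPoint inserts the world-space point, then requires a static mesh component to continue.
; A box overlap checks for nearby decal components; if none are found, it spawns an attached decal with fade screen size zero, keeping it visible at distance.
; Both outcomes print debug strings.
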(event `Add Decal Point`
  (params (Index :type Integer) (`Point Location` :type "Vector Structure") (`Decal Rotation` :type "Rotator Structure") (`Scene Component` :type "SceneComponent Object Reference"))
  (`SplineComponent.AddSplinePointAtIndex` (`self.Spline`) `Point Location` Index "World" true)
  (bind _asstatic_mesh_component (cast `StaticMeshComponent` `Scene Component`))
  (bind (_outcomponents _returnvalue) (`KismetSystemLibrary.BoxOverlapComponents` `Point Location` (* (`self.DecalSize`) 10) (`|MakeArray` "ObjectTypeQuery1" "ObjectTypeQuery2" :!type "EObjectTypeQuery Enum") "/Script/Engine.DecalComponent"))
  (if _returnvalue
    (`KismetSystemLibrary.PrintString` "DECAL")
    (else
      (bind _returnvalue_2 (`GameplayStatics.SpawnDecalAttached` "/Game/Materials/whiteboard/MarkerDecal.MarkerDecal" (`self.DecalSize`) _asstatic_mesh_component "None" `Point Location` `Decal Rotation` "KeepWorldPosition"))
      (`DecalComponent.SetFadeScreenSize` _returnvalue_2 0.0) ; Allows player to see decal from anywhere
      (`KismetSystemLibrary.PrintString` "Decal Drawn"))))

(fn `UserConstructionScript`)