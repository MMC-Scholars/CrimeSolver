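; Whiteboard actor that supports runtime drawing by painting into a shared render target, RT_Whiteboard.
; On BeginPlay it creates a dynamic instance of M_Marker and clears the render target to black.
; The Draw and Erase events pass a 2D location into the marker's DrawLocation parameter, then draw that material onto the target.
; Erase is currently identical to Draw, using the same material, and the material parameter collection nodes are unconnected.
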(event `self.ReceiveBeginPlay`
  (`parent.ReceiveBeginPlay`)
  (bind _returnvalue (`KismetMaterialLibrary.CreateDynamicMaterialInstance` "/Game/Materials/marker_and_eraser/M_Marker.M_Marker"))
  (set `self.WhiteboardMarker_MI` _returnvalue)
  (`KismetRenderingLibrary.ClearRenderTarget2D` "/Game/Materials/marker_and_eraser/RT_Whiteboard.RT_Whiteboard"))

(event `Draw`
  (params (`Drawn Location` :type "Vector2D Structure"))
  (bind _whiteboardmarker_mi (`self.WhiteboardMarker_MI`))
  (`MaterialInstanceDynamic.SetVectorParameterValue` _whiteboardmarker_mi "DrawLocation" (`KismetMathLibrary.Conv_VectorToLinearColor` (`KismetMathLibrary.Conv_Vector2DToVector` `Drawn Location`)))
  (`KismetRenderingLibrary.DrawMaterialToRenderTarget` "/Game/Materials/marker_and_eraser/RT_Whiteboard.RT_Whiteboard" _whiteboardmarker_mi))

(event `Erase`
  (params (`Erase Location` :type "Vector2D Structure"))
  (bind _whiteboardmarker_mi (`self.WhiteboardMarker_MI`))
  (`MaterialInstanceDynamic.SetVectorParameterValue` _whiteboardmarker_mi "DrawLocation" (`KismetMathLibrary.Conv_VectorToLinearColor` (`KismetMathLibrary.Conv_Vector2DToVector` `Erase Location`)))
  (`KismetRenderingLibrary.DrawMaterialToRenderTarget` "/Game/Materials/marker_and_eraser/RT_Whiteboard.RT_Whiteboard" _whiteboardmarker_mi))

(fn `UserConstructionScript`
  (`parent.UserConstructionScript`))