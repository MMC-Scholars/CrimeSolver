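; Desktop first-person player character that moves, crouches, interacts with objects and handles an inventory of tools.
; Movement input is projected onto the navmesh, with velocity cancelling at its edges, while a timeline blends capsule, eye height and speed for crouching.
; InventorySystem receives GameMode default tools and handles slot switching, aiming, use, and tap-to-toss or hold-to-throw drops.
; Camera traces drive InteractionBPI calls and a FindEvidence query.
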(event `self.ReceiveBeginPlay`
  (set `self.vLastNavmeshLocation` (`NavigationSystemV1.K2_ProjectPointToNavigation` (`SceneComponent.K2_GetComponentLocation` (`self.Feet`))))
  (bind _returnvalue (`AddComponent|NODE_AddChildActorComponent-1` :`self` (`GameplayStatics.GetPlayerCameraManager` 0) :`RelativeTransform` (`KismetMathLibrary.MakeTransform` (0.0 0.0 0.0)))) ; Make hand move with camera rotation
  (`SceneComponent.K2_AttachToComponent` (`self.Hand`) _returnvalue "None" "KeepRelative" "KeepRelative" "KeepRelative" true)
  (`self.Spawn Tools`)
  (set `/Game/Blueprints/DesktopPawn/Inventory.tDefaultTransform` (`SceneComponent.GetRelativeTransform` (`self.Hand`)) (`self.InventorySystem`))
  (bind _returnvalue_2 (`|CreateWidget` "/Game/Blueprints/PlayerHUD.PlayerHUD_C" (`GameplayStatics.GetPlayerController` 0)))
  (bind _output_get (set `self.StandardHUD` _returnvalue_2))
  (`UserWidget.AddToViewport` _output_get 0)
  (add `self.CancelThrow` (`|CreateDelegate` :!event `Cancelled Throw Exec Portal`)))

(event `InputAction|Crouch`
  (params (Key :type "Key Structure"))
  (bind _bistogglecrouchenabled (`self.bIsToggleCrouchEnabled`))
  (bind _biscrouching (`self.bIsCrouching`))
  ;[1 1 1] Crouching
  (:`Pressed`
    ;;[1 1 1] Toggle Crouch
    (if _bistogglecrouchenabled
      (bind _output_get (set `self.bIsCrouching` (not _biscrouching) :!label _label))
      (`self.Smooth Crouch` _output_get)
      (else
        ;;[1 1 1] Prevent Inverted Crouching
        (if (not _biscrouching)
          (goto _label)))))
  (:`Released`
    (if _bistogglecrouchenabled
      _
      (elif _biscrouching
        (goto _label)))))

(event `Smooth Crouch`
  (params (`Is Crouching` :type Boolean))
  ;[1 1 1] Crouching
  (if `Is Crouching`
    (bind (_direction _lerp_alpha) (`Timeline|Interpolate Crouch` :!label _label_2)
      (:`Update`
        (`self.ChangeMovement` _lerp_alpha)))
    (else
      (bind _canstand (`self.CanStandUp`))
      (if _canstand
        (goto _label_2 :!via `Reverse`)))))

(event `InputAxis|Strafe-Left-Right`
  (params (AxisValue :type "Float (single-precision)"))
  ;[1 1 1] Character Movement
  (`self.MoveAlongNavMesh` :!label _label_3)
  ;;[1 1 1] Correct capsule half-height after uncrouching under an object
  (if (and (!= (`CapsuleComponent.CapsuleHalfHeight` (`self.CapsuleComponent`)) (`self.fStandingHalfHeight`)) (not (`self.bIsCrouching`)))
    (`self.Smooth Crouch` false)))

(event `InputAxis|Forward-Backward`
  (params (AxisValue :type "Float (single-precision)"))
  ;[1 1 1] Character Movement
  (goto _label_3))

(event `MoveAlongNavMesh`
  (bind _returnvalue (`self.GetInputAxisValue`))
  (bind _returnvalue_2 (`self.GetInputAxisValue`))
  (bind _charactermovement (`self.CharacterMovement`))
  (bind (_vlastnavmeshlocation_x _vlastnavmeshlocation_y _vlastnavmeshlocation_z) (`KismetMathLibrary.BreakVector` (`self.vLastNavmeshLocation`)))
  (bind _feet (`self.Feet`))
  (bind _returnvalue_3 (`SceneComponent.K2_GetComponentLocation` _feet))
  (bind _returnvalue_4 (`KismetMathLibrary.Hypotenuse` _returnvalue _returnvalue_2))
  (bind _velocity (`MovementComponent.Velocity` _charactermovement))
  (bind _returnvalue_5 (+ (* (`SceneComponent.GetForwardVector` _feet) _returnvalue) (* (`SceneComponent.GetRightVector` _feet) _returnvalue_2)))
  (bind (_projectedlocation _returnvalue_6) (`NavigationSystemV1.K2_ProjectPointToNavigation` (+ _returnvalue_3 _returnvalue_5)))
  (bind _returnvalue_7 (- _projectedlocation (`KismetMathLibrary.MakeVector` (.x _returnvalue_3) (.y _returnvalue_3) _vlastnavmeshlocation_z)))
  (bind _returnvalue_8 (`KismetMathLibrary.GetDirectionUnitVector` _returnvalue_5 _returnvalue_7))
  ;[1 1 1] Character Movement
  (if _returnvalue_6
    ;;[1 1 1] Velocity cusioning to prevent oscilating when running into the end of the navigation mesh
    (set `MovementComponent.Velocity` (select `bool` (`KismetMathLibrary.NearlyEqual_FloatFloat` (`KismetMathLibrary.VSize` _returnvalue_7) _returnvalue_4 2e-05) :`false` (- _velocity (* _returnvalue_8 (`KismetMathLibrary.Dot_VectorVector` _velocity _returnvalue_8))) :`true` _velocity) _charactermovement)
    (set `self.vLastNavmeshLocation` _projectedlocation) ; For more accurate positioning
    (`self.AddMovementInput` _returnvalue_7 _returnvalue_4)))

(event `InputAxis|Rotate-Left-Right`
  (params (AxisValue :type "Float (single-precision)"))
  (bind _returnvalue (* AxisValue (`self.fMouseXSens`)))
  ;[1 1 1] Mouse Movement Input
  (bind _result (`/Engine/EditorBlueprintResources/StandardMacros.NegateFloat` _returnvalue)
    (:`  `
      (`self.AddControllerYawInput` (select `bool` (`self.bIsXAxisInverted`) :`false` _returnvalue :`true` _result)))))

(event `InputAxis|Look-Up-Down`
  (params (AxisValue :type "Float (single-precision)"))
  (bind _returnvalue (* AxisValue (`self.fMouseYSens`)))
  ;[1 1 1] Mouse Movement Input
  (bind _result (`/Engine/EditorBlueprintResources/StandardMacros.NegateFloat` _returnvalue)
    (:`  `
      (`self.AddControllerPitchInput` (select `bool` (`self.bIsYAxisInverted`) :`false` _returnvalue :`true` _result)))))

(event `InputAction|Drop`
  (params (Key :type "Key Structure"))
  (:`Pressed`
    (goto _label :!via `Close`))
  (:`Released`
    (goto _label :!via `Open`)))

(event `InputAxis|ScrollInventory`
  (params (AxisValue :type "Float (single-precision)"))
  (bind _returnvalue (`KismetMathLibrary.Round` AxisValue))
  (if (!= _returnvalue 0)
    (`/Engine/EditorBlueprintResources/StandardMacros.Gate` false :!label _label
      (:`Exit`
        (if (not (or (`self.bIsAiming`) (`self.bIsThrowingItem`))) :!label _label_2
          (bind _newinventoryslot (`self.PickSlot` (stale `InputAction|Inventory` Key) _returnvalue))
          (`self.ChangeTools` _newinventoryslot))))))

(event `InputAction|Inventory`
  (params (Key :type "Key Structure"))
  (:`Pressed`
    (goto _label_2)))

(event `InputAction|Aim`
  (params (Key :type "Key Structure"))
  (bind _inventorysystem (`self.InventorySystem`))
  (bind _bisthrowingitem (`self.bIsThrowingItem`))
  (bind _icurrentinventoryslot (`self.iCurrentInventorySlot`))
  (:`Pressed`
    (if _bisthrowingitem
      (set `self.bIsThrowingItem` false) ; Cancel Throw
      (`self.CancelThrow`)
      (else
        (set `self.bIsAiming` true)
        (`/Game/Blueprints/DesktopPawn/Inventory.Aim In` _inventorysystem _icurrentinventoryslot)
        (`/Engine/EditorBlueprintResources/StandardMacros.Gate` false :!via `Open` :!label _label_3) ; Allow zooming when aiming
      )))
  (:`Released`
    (if (not _bisthrowingitem)
      (set `self.bIsAiming` false)
      (`/Game/Blueprints/DesktopPawn/Inventory.Aim Out` _inventorysystem _icurrentinventoryslot)
      (goto _label_3 :!via `Close`))))

(event `InputAction|Fire`
  (params (Key :type "Key Structure"))
  (:`Pressed`
    (`/Game/Blueprints/DesktopPawn/Inventory.Use` (`self.InventorySystem`) (`self.iCurrentInventorySlot`))))

(event `InputAction|Interact`
  (params (Key :type "Key Structure"))
  (bind _returnvalue (`GameplayStatics.GetPlayerCameraManager` 0))
  (bind _bisaiming (`self.bIsAiming`))
  (bind _returnvalue_2 (`PlayerCameraManager.GetCameraLocation` _returnvalue))
  (:`Pressed`
    (if (not _bisaiming)
      (bind _outhit (`KismetSystemLibrary.LineTraceSingleForObjects` _returnvalue_2 (+ _returnvalue_2 (* (`KismetMathLibrary.GetForwardVector` (`PlayerCameraManager.GetCameraRotation` _returnvalue)) (`self.fInteractionDistance`))) (`|MakeArray` "ObjectTypeQuery1" "ObjectTypeQuery2" "ObjectTypeQuery4" "ObjectTypeQuery7" :!type "EObjectTypeQuery Enum") false (`/Game/Blueprints/DesktopPawn/Inventory.InventoryItems` (`self.InventorySystem`))))
      (bind (_bblockinghit _binitialoverlap _time _distance _location _impactpoint _normal _impactnormal _physmat _hitactor) (`GameplayStatics.BreakHitResult` _outhit))
      (if (and _bblockinghit (`KismetSystemLibrary.DoesImplementInterface` _hitactor "/Game/Blueprints/InteractionBPI.InteractionBPI_C"))
        (message `/Game/Blueprints/InteractionBPI.InteractWithObject` _hitactor self _impactpoint _impactnormal))))
  (:`Released`
    (if (not _bisaiming)
      (message `/Game/Blueprints/InteractionBPI.StopInteractWithObject` _hitactor))))

(event `InputAction|Drop`
  (params (Key :type "Key Structure"))
  (bind _fthrowingholdtime (`self.fThrowingHoldTime`))
  (bind _returnvalue (and (not (`self.bIsAiming`)) (`/Game/Blueprints/DesktopPawn/Inventory.bAreSlotsSwitched` (`self.InventorySystem`))))
  (:`Pressed`
    (if _returnvalue
      (`KismetSystemLibrary.Delay` (+ _fthrowingholdtime 0.005))
      (set `self.bIsThrowingItem` (> (`PlayerController.GetInputKeyTimeDown` (`GameplayStatics.GetPlayerController` 0) Key) _fthrowingholdtime))
      (else
        (goto _label_4 :!via `Close`))))
  (:`Released`
    (`|ExecutionSequence`
      (:`then_0`
        (`/Engine/EditorBlueprintResources/StandardMacros.Gate` false :!label _label_4
          (:`Exit`
            (if _returnvalue
              (`/Game/Blueprints/DesktopPawn/Inventory.Launch Item` (`self.InventorySystem`) (`self.iCurrentInventorySlot`) (select `bool` (`self.bIsThrowingItem`) :`false` (`self.fTossingSpeed`) :`true` (`self.fThrowingSpeed`)) (`self.fThrowingAngle`))
              (set `self.bIsThrowingItem` false)))))
      (:`then_1`
        (goto _label_4 :!via `Open`)))))

(event `Cancelled Throw Exec Portal`
  (goto _label_4 :!via `Close`))

(fn `CanStandUp`
  (returns (CanStand :type Boolean))
  (bind _fstandinghalfheight (`self.fStandingHalfHeight`))
  (bind (_outactors _returnvalue) (`KismetSystemLibrary.CapsuleOverlapActors` (+ (- (`SceneComponent.K2_GetComponentLocation` (`self.Feet`)) (`KismetMathLibrary.MakeVector` 0.0 0.0 (`self.fFeetCollisionDisplacement`))) (`KismetMathLibrary.MakeVector` 0.0 0.0 _fstandinghalfheight)) (`CapsuleComponent.CapsuleRadius` (`self.CapsuleComponent`)) _fstandinghalfheight (`|MakeArray` "ObjectTypeQuery1" "ObjectTypeQuery2" :!type "EObjectTypeQuery Enum") null (`/Game/Blueprints/DesktopPawn/Inventory.InventoryItems` (`self.InventorySystem`))))
  (return (not _returnvalue)))

(fn `ChangeMovement`
  (params (`LERP Alpha` :type "Float (double-precision)") (`Movement Index` :type Integer))
  (bind _fwalkspeed (`self.fWalkSpeed`))
  (bind _returnvalue (`KismetMathLibrary.Lerp` (`self.fStandingHalfHeight`) (`self.fCrouchingHalfHeight`) `LERP Alpha`))
  (`|ExecutionSequence`
    (:`then_0`
      (`CapsuleComponent.SetCapsuleHalfHeight` (`self.CapsuleComponent`) _returnvalue true)
      (`SceneComponent.K2_SetRelativeLocation` (`self.Feet`) (`KismetMathLibrary.MakeVector` 0.0 0.0 (- (`self.fFeetCollisionDisplacement`) _returnvalue)) false true))
    (:`then_1`
      (set `CharacterMovementComponent.MaxWalkSpeed` (`KismetMathLibrary.Lerp` _fwalkspeed (* _fwalkspeed (`self.fCrouchSpeedMultiplier`)) `LERP Alpha`) (`self.CharacterMovement`)) ; This is move speed
    )
    (:`then_2`
      (set `self.BaseEyeHeight` (`KismetMathLibrary.Lerp` (`self.fStandingEyeHeight`) (`self.fCrouchingEyeHeight`) `LERP Alpha`)))))

(fn `ChangeTools`
  (params (NewInventorySlot :type Integer))
  (bind _icurrentinventoryslot (`self.iCurrentInventorySlot`))
  (if (!= NewInventorySlot _icurrentinventoryslot)
    (`/Game/Blueprints/DesktopPawn/Inventory.Deselect Item` (`self.InventorySystem`) NewInventorySlot _icurrentinventoryslot)
    (`/Game/Blueprints/DesktopPawn/Inventory.Select Item` (`self.InventorySystem`) NewInventorySlot)
    (bind _output_get (set `self.iCurrentInventorySlot` NewInventorySlot))
    (`KismetSystemLibrary.PrintString` (`KismetStringLibrary.Conv_IntToString` _output_get))))

(fn `FindEvidence`
  (returns (EvidenceHit :type "Array of /Game/Blueprints/Interactables/Items/Evidence/Evidence Object Reference") (WasEvidenceFound :type Boolean))
  (locals (fEvidenceFOV :type "Float (double-precision)" :default 7.5) (ObjectWorldTypes :type "Array of EObjectTypeQuery Enum") (ViewedEvidence :type "Array of /Game/Blueprints/Interactables/Items/Evidence/Evidence Object Reference"))
  (bind _returnvalue (`GameplayStatics.GetPlayerCameraManager` 0))
  (bind _viewedevidence (`local.ViewedEvidence`))
  (bind _returnvalue_2 (`PlayerCameraManager.GetCameraLocation` _returnvalue))
  ;[1 1 1] Sphere tracing extended 1.5 meters infront of the headset/player
  (bind _outhits (`KismetSystemLibrary.SphereTraceMultiForObjects` _returnvalue_2 (+ _returnvalue_2 (* (`KismetMathLibrary.GetForwardVector` (`PlayerCameraManager.GetCameraRotation` _returnvalue)) 150.0)) (`local.fEvidenceFOV`) (`local.ObjectWorldTypes`)))
  (for _array_element _outhits
    ;[1 1 1] Create array of identified evidence
    (bind _asevidence (cast `/Game/Blueprints/Interactables/Items/Evidence/Evidence` (`.HitActor` (`GameplayStatics.BreakHitResult` _array_element))))
    (`KismetArrayLibrary.Array_Add` _viewedevidence _asevidence))
  (return _viewedevidence (> (`KismetArrayLibrary.Array_Length` _viewedevidence) 0)))

(fn `PickSlot`
  (params (KeyInput :type "Key Structure" :default "None") (`Axis Value` :type Integer))
  (returns (NewInventorySlot :type Integer))
  (locals (aKeyPresses :type "Array of Key Structure") (iNumofSlots :type Integer :default 9) (iNewSlot :type Integer) (iAxisValue :type Integer))
  (bind _iaxisvalue (`local.iAxisValue`))
  (bind _icurrentinventoryslot (`self.iCurrentInventorySlot`))
  (bind _output_get (set `local.iAxisValue` `Axis Value`))
  (if (== _output_get 0)
    (set `local.iNewSlot` (`KismetArrayLibrary.Array_Find` (`local.aKeyPresses`) KeyInput))
    (else
      ;[1 1 1] Scrollwheel
      (if (> _iaxisvalue 0)
        (if (== (`local.iNumOfSlots`) _icurrentinventoryslot)
          (set `local.iNewSlot` 0) ; Overflow to 0
          (else
            (set `local.iNewSlot` (+ (`self.iCurrentInventorySlot`) (`KismetMathLibrary.SignOfInteger` _iaxisvalue)) :!label _label) ; Add or Subtract 1
          ))
        (elif (== _icurrentinventoryslot 0)
          (set `local.iNewSlot` (`local.iNumOfSlots`)) ; Overflow to Max
          (else
            (goto _label))))))
  (return (`local.iNewSlot`)))

(fn `PickUpItem`
  (params (Item :type "/Game/Blueprints/Interactables/Items/Item Object Reference"))
  (bind _icurrentinventoryslot (`self.iCurrentInventorySlot`))
  (bind (_added_item _itemslot) (`/Game/Blueprints/DesktopPawn/Inventory.AddItemToInventory` (`self.InventorySystem`) Item _icurrentinventoryslot))
  (if (== _icurrentinventoryslot _itemslot)
    (`/Game/Blueprints/DesktopPawn/Inventory.Select Item` (`self.InventorySystem`) _icurrentinventoryslot)))

(fn `SpaceInInventory`
  (returns (IsSpaceInInventory :type Boolean))
  (locals (bSpaceInInventory :type Boolean))
  (for _index (range 1 10)
    (set `local.bSpaceInInventory` (or (not (`|GetArrayItem` (`/Game/Blueprints/DesktopPawn/Inventory.bIsSlotFilled` (`self.InventorySystem`)) _index)) (`local.bSpaceInInventory`))))
  (return (`local.bSpaceInInventory`)))

(fn `Spawn Tools`
  ;[1 1 1] Spawn tools
  (bind _asgame_mode_bp (cast `/Game/Blueprints/GameModeBP` (`GameplayStatics.GetGameMode`))
    (:`then`
      (set `/Game/Blueprints/DesktopPawn/Inventory.InventoryOwner` self (`self.InventorySystem`))
      (for (_array_element _array_index) (`/Game/Blueprints/GameModeBP.DefaultInventory` _asgame_mode_bp)
        (bind _returnvalue (`|SpawnActorFromClass` _array_element (`self.GetTransform`) "AlwaysSpawn" "OverrideRootScale" self null))
        (`/Game/Blueprints/DesktopPawn/Inventory.AddItemToInventory` (`self.InventorySystem`) _returnvalue (+ _array_index 1))))
    (:`CastFailed`
      (`KismetSystemLibrary.QuitGame` null "Quit") ; Shouldn't Trigger
    )))

(fn `UserConstructionScript`
  (bind _capsulecomponent (`self.CapsuleComponent`))
  (bind (_relativelocation_x _relativelocation_y _relativelocation_z) (`KismetMathLibrary.BreakVector` (`SceneComponent.RelativeLocation` (`self.Feet`))))
  (`CapsuleComponent.SetCapsuleHalfHeight` _capsulecomponent (`self.fStandingHalfHeight`) true)
  (set `self.fFeetCollisionDisplacement` (+ (`CapsuleComponent.CapsuleHalfHeight` _capsulecomponent) _relativelocation_z)))