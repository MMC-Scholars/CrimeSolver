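; Inventory component for the desktop pawn that spawns and stores the player's tools.
; On BeginPlay it spawns every tool type listed by GameModeBP at the owner's transform with collision off and hidden, quitting the game if that cast fails.
; ChangeTools only starts a move to a stored home position and rotation when a change is needed and the slot is nonzero; it does not yet swap tools.
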(event `self.ReceiveBeginPlay`
  ;[1 1 1] Spawn tools
  (bind _asgame_mode_bp (cast `/Game/Blueprints/GameModeBP` (`GameplayStatics.GetGameMode`))
    (:`then`
      (for _array_element (`/Game/Blueprints/GameModeBP.ToolTypes` _asgame_mode_bp)
        (bind _returnvalue (`|SpawnActorFromClass` _array_element (`Actor.GetTransform` (`self.GetOwner`)) "AdjustIfPossibleButAlwaysSpawn" "OverrideRootScale" null null))
        (`Actor.SetActorEnableCollision` _returnvalue false)
        (`Actor.SetActorHiddenInGame` _returnvalue true)
        (`KismetArrayLibrary.Array_Add` (`self.Tools`) _returnvalue)))
    (:`CastFailed`
      (`KismetSystemLibrary.QuitGame` null "Quit") ; Shouldn't Trigger
    )))

(event `Change Tools`
  (params (`Tool Slot` :type Integer) (`Change Needed` :type Boolean))
  (if `Change Needed`
    (if (!= `Tool Slot` 0)
      (`KismetSystemLibrary.MoveComponentTo` null (`self.vHomePosition`) (`self.rHomeRotation`)))))