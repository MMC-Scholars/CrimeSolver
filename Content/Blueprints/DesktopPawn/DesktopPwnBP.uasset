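; Player pawn for desktop play, with navmesh-bound walking, mouse look and toggle or hold crouching.
; Movement axes offset the last navmesh point, project it back onto the navmesh, then teleport the pawn above it by capsule height.
; Crouch changes speed and target height, which the capsule approaches stepwise during movement updates.
; The construction script nudges the pawn upward until its capsule clears overlapping objects.
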(event `self.ReceiveBeginPlay`
  (set `self.fTimeElapsed` 0.0)
  (set `self.vLastNavLoc` (`NavigationSystemV1.K2_ProjectPointToNavigation` (`SceneComponent.K2_GetComponentLocation` (`self.Capsule`)))))

(event `InputAction|Crouch`
  (params (Key :type "Key Structure"))
  (bind _btogglecrouch (`self.bToggleCrouch`))
  (bind _biscrouching (`self.bIsCrouching`))
  ;[1 1 1] Crouching
  (:`Pressed`
    ;;[1 1 1] Toggle Crouch
    (if _btogglecrouch
      (bind _output_get (set `self.bIsCrouching` (not _biscrouching) :!label _label))
      ;;[1 1 1] Speed and Height Changes
      (set `self.fMoveSpeedMultiplier` (select `bool` _output_get :`false` 3.0 :`true` 1.5 :!type "Float (single-precision)"))
      (set `self.fHalfHeight` (select `bool` _output_get :`false` 96.0 :`true` 52.0 :!type "Float (single-precision)"))
      (else
        ;;[1 1 1] Prevent Inverted Crouching
        (if (not _biscrouching)
          (goto _label)))))
  (:`Released`
    (if _btogglecrouch
      _
      (elif _biscrouching
        (goto _label)))))

(event `InputAxis|Forward-Backward`
  (params (AxisValue :type "Float (single-precision)"))
  ;[1 1 1] Movement bound to Navigational Mesh Bounds Volume
  (bind _navmesh_position (`self.GetNavmeshPos` (`self.GetActorForwardVector`) AxisValue))
  (bind _world_position (`self.NavmeshToWorldPos` _navmesh_position))
  ;;[1 1 1] Move pawn and update variables
  (`self.K2_SetActorLocation` _world_position)
  (set `self.vLastNavLoc` _navmesh_position)
  (set `self.fTimeElapsed` (`.PartialSeconds` (`GameplayStatics.GetAccurateRealTime`))))

(event `InputAxis|Strafe-Left-Right`
  (params (AxisValue :type "Float (single-precision)"))
  ;[1 1 1] Movement bound to Navigational Mesh Bounds Volume
  (bind _navmesh_position (`self.GetNavmeshPos` (`self.GetActorRightVector`) AxisValue))
  (bind _world_position (`self.NavmeshToWorldPos` _navmesh_position))
  ;;[1 1 1] Move pawn and update variables
  (`self.K2_SetActorLocation` _world_position)
  (set `self.vLastNavLoc` _navmesh_position)
  (set `self.fTimeElapsed` (`.PartialSeconds` (`GameplayStatics.GetAccurateRealTime`))))

(event `InputAxis|Rotate-Left-Right`
  (params (AxisValue :type "Float (single-precision)"))
  (bind _returnvalue (* AxisValue (`self.fMouseXSens`)))
  ;[1 1 1] Mouse Movement Input
  (bind _result (`/Engine/EditorBlueprintResources/StandardMacros.NegateFloat` _returnvalue)
    (:`  `
      (`self.AddControllerYawInput` (select `bool` (`self.bInvertXAxis`) :`false` _returnvalue :`true` _result)))))

(event `InputAxis|Look-Up-Down`
  (params (AxisValue :type "Float (single-precision)"))
  (bind _returnvalue (* AxisValue (`self.fMouseYSens`)))
  ;[1 1 1] Mouse Movement Input
  (bind _result (`/Engine/EditorBlueprintResources/StandardMacros.NegateFloat` _returnvalue)
    (:`  `
      (`self.AddControllerPitchInput` (select `bool` (`self.bInvertYAxis`) :`false` _returnvalue :`true` _result)))))

(fn `GetNavmeshPos`
  (params (`Initial Direction` :type "Vector Structure") (`Axis Value` :type "Float (double-precision)"))
  (returns (`Navmesh Position` :type "Vector Structure"))
  (return (`NavigationSystemV1.K2_ProjectPointToNavigation` (+ (* (* `Initial Direction` `Axis Value`) (`self.fMoveSpeedMultiplier`)) (`self.vLastNavLoc`)))))

(fn `NavmeshToWorldPos`
  (params (`Navmesh Position` :type "Vector Structure"))
  (returns (`World Position` :type "Vector Structure"))
  (bind _fhalfheight (`self.fHalfHeight`))
  (bind _returnvalue (`CapsuleComponent.GetUnscaledCapsuleHalfHeight` (`self.Capsule`)))
  ;[1 1 1] Process Crouching Height Changes
  (if (not (== _returnvalue _fhalfheight))
    (`CapsuleComponent.SetCapsuleHalfHeight` (`self.Capsule`) (- _returnvalue (select `bool` (> _returnvalue _fhalfheight) :`false` -2.0 :`true` 2.0 :!type "Float (single-precision)")) true))
  (return (+ (`KismetMathLibrary.MakeVector` 0.0 0.0 (`CapsuleComponent.GetScaledCapsuleHalfHeight_WithoutHemisphere` (`self.Capsule`))) `Navmesh Position`)))

(fn `UserConstructionScript`
  (locals (ObjectTypes :type "Array of EObjectTypeQuery Enum") (CapsulePos :type "Transform Structure"))
  (bind _capsule (`self.Capsule`))
  (bind _capsule_2 (`self.Capsule`))
  (set `self.bUseControllerRotationYaw` true)
  (`self.K2_SetActorLocationAndRotation` (`SceneComponent.K2_GetComponentLocation` _capsule) (`SceneComponent.K2_GetComponentRotation` _capsule))
  ;[1 1 1] Teleports pawn above any objects overlapping capsule hitbox at the end of drag
  (`self.Do While` (stale _returnvalue)
    (:`Loop Body`
      (bind (_outactors _returnvalue) (`KismetSystemLibrary.ComponentOverlapActors` _capsule_2 (`SceneComponent.K2_GetComponentToWorld` _capsule_2) (`local.ObjectTypes`))) ; May have to add "Actors to Ignore" in future
      (if _returnvalue
        (`self.K2_AddActorWorldOffset` (0.0 0.0 1.0) false true)))))