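; Player pawn for desktop play, with mouse look, crouching, a tool inventory and object interaction.
; Movement projects each step onto the navmesh and sets location at capsule height, easing crouch height during moves.
; An Inventory component handles GameMode-defined tools; right-mouse gates restrict switching, dropping and line-traced InteractionBPI interaction while aiming.
; FindEvidence sphere-traces for Evidence actors, and the construction script lifts the pawn out of overlaps.
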(event `self.ReceiveBeginPlay`
  (set `self.fTimeElapsed` 0.0)
  (set `self.vLastNavmeshPos` (`NavigationSystemV1.K2_ProjectPointToNavigation` (`SceneComponent.K2_GetComponentLocation` (`self.Capsule`))))
  (set `self.fCurrentMoveSpeed` (`self.fMovementMultiplier`))
  (`self.Spawn Tools`)
  (set `/Game/Blueprints/DesktopPawn/Inventory.tDefaultTransform` (`SceneComponent.GetRelativeTransform` (`self.Hand`)) (`self.Inventory`))
  (bind _returnvalue (`|CreateWidget` "/Game/Blueprints/PlayerHUD.PlayerHUD_C" (`GameplayStatics.GetPlayerController` 0)))
  (bind _output_get (set `self.StandardHUD` _returnvalue))
  (`UserWidget.AddToViewport` _output_get 0)
  (`Widget.SetVisibility` _output_get "Hidden"))

(event `InputAction|Crouch`
  (params (Key :type "Key Structure"))
  (bind _fmovementmultiplier (`self.fMovementMultiplier`))
  (bind _bistogglecrouchenabled (`self.bIsToggleCrouchEnabled`))
  (bind _biscrouching (`self.bIsCrouching`))
  ;[1 1 1] Crouching
  (:`Pressed`
    ;;[1 1 1] Toggle Crouch
    (if _bistogglecrouchenabled
      (bind _output_get (set `self.bIsCrouching` (not _biscrouching) :!label _label))
      ;;[1 1 1] Speed and Height Changes
      (set `self.fCurrentMoveSpeed` (select `bool` _output_get :`false` _fmovementmultiplier :`true` (* _fmovementmultiplier 0.5)))
      (set `self.fCapsuleHalfHeight` (select `bool` _output_get :`false` 96.0 :`true` 52.0 :!type "Float (single-precision)")) ; TODO: Will be changed if using model
      (else
        ;;[1 1 1] Prevent Inverted Crouching
        (if (not _biscrouching)
          (goto _label)))))
  (:`Released`
    (if _bistogglecrouchenabled
      _
      (elif _biscrouching
        (goto _label)))))

(event `InputAxis|Forward-Backward`
  (params (AxisValue :type "Float (single-precision)"))
  (bind (_seconds _partialseconds) (`GameplayStatics.GetAccurateRealTime`))
  ;[1 1 1] Movement bound to Navigational Mesh Bounds Volume
  (bind _navmesh_position (`self.Get Navmesh Pos` (`self.GetActorForwardVector`) AxisValue))
  (bind _world_position (`self.Navmesh To World Pos` _navmesh_position))
  ;;[1 1 1] Move pawn and update variables
  (`self.K2_SetActorLocation` _world_position)
  (set `self.vLastNavmeshPos` _navmesh_position)
  (set `self.fTimeElapsed` (+ (`KismetMathLibrary.Conv_IntToDouble` _seconds) _partialseconds)))

(event `InputAxis|Strafe-Left-Right`
  (params (AxisValue :type "Float (single-precision)"))
  (bind (_seconds _partialseconds) (`GameplayStatics.GetAccurateRealTime`))
  ;[1 1 1] Movement bound to Navigational Mesh Bounds Volume
  (bind _navmesh_position (`self.Get Navmesh Pos` (`self.GetActorRightVector`) AxisValue))
  (bind _world_position (`self.Navmesh To World Pos` _navmesh_position))
  ;;[1 1 1] Move pawn and update variables
  (`self.K2_SetActorLocation` _world_position)
  (set `self.vLastNavmeshPos` _navmesh_position)
  (set `self.fTimeElapsed` (+ (`KismetMathLibrary.Conv_IntToDouble` _seconds) _partialseconds)))

(event `InputAxis|Rotate-Left-Right`
  (params (AxisValue :type "Float (single-precision)"))
  (bind _returnvalue (* AxisValue (`self.fMouseXSens`)))
  ;[1 1 1] Mouse Movement Input
  (bind _result (`/Engine/EditorBlueprintResources/StandardMacros.NegateFloat` _returnvalue)
    (:`  `
      (`self.AddControllerYawInput` (select `bool` (`self.bIsXAxisInverted`) :`false` _returnvalue :`true` _result)))))

(event `InputAxis|Look-Up-Down`
  (params (AxisValue :type "Float (single-precision)"))
  (bind _returnvalue (* AxisValue (`self.fMouseYSens`)))
  ;[1 1 1] Mouse Movement Input
  (bind _result (`/Engine/EditorBlueprintResources/StandardMacros.NegateFloat` _returnvalue)
    (:`  `
      (`self.AddControllerPitchInput` (select `bool` (`self.bIsYAxisInverted`) :`false` _returnvalue :`true` _result)))))

(event `InputAxis|ScrollInventory`
  (params (AxisValue :type "Float (single-precision)"))
  (bind _returnvalue (`KismetMathLibrary.Round` AxisValue))
  (if (!= _returnvalue 0)
    (`|ExecutionSequence`
      (:`then_0`
        (`/Engine/EditorBlueprintResources/StandardMacros.Gate` false :!label _label ; Prevent switching when aiming
          (:`Exit`
            (bind _new_tool_slot (`self.Pick Slot` (stale `InputAction|Inventory` Key) _returnvalue))
            (`self.Change Tools` _new_tool_slot)))))))

(event `InputAction|Inventory`
  (params (Key :type "Key Structure"))
  (:`Pressed`
    (goto _label)))

(event `Key|RightMouseButton`
  (params (Key :type "Key Structure"))
  (:`Pressed`
    (goto _label :!via `Close`))
  (:`Released`
    (goto _label :!via `Open`)))

(event `InputAction|Aim`
  (params (Key :type "Key Structure"))
  (bind _inventory (`self.Inventory`))
  (bind _icurrentinventoryslot (`self.iCurrentInventorySlot`))
  (:`Pressed`
    (`/Game/Blueprints/DesktopPawn/Inventory.Aim In` _inventory _icurrentinventoryslot)
    (`/Engine/EditorBlueprintResources/StandardMacros.Gate` false :!via `Open` :!label _label_2) ; Allow zooming when aiming
  )
  (:`Released`
    (`/Game/Blueprints/DesktopPawn/Inventory.Aim Out` _inventory _icurrentinventoryslot)
    (goto _label_2 :!via `Close`)))

(event `InputAction|Fire`
  (params (Key :type "Key Structure"))
  (:`Pressed`
    (`/Game/Blueprints/DesktopPawn/Inventory.Use` (`self.Inventory`) (`self.iCurrentInventorySlot`))))

(event `Key|RightMouseButton`
  (params (Key :type "Key Structure"))
  (bind _camera (`self.Camera`))
  (bind _returnvalue (`SceneComponent.K2_GetComponentLocation` _camera))
  (:`Pressed`
    (goto _label_3 :!via `Close`))
  (:`Released`
    (goto _label_3 :!via `Open`)))

(event `InputAction|Interact`
  (params (Key :type "Key Structure"))
  (bind _camera (`self.Camera`))
  (bind _returnvalue (`SceneComponent.K2_GetComponentLocation` _camera))
  (:`Pressed`
    (`/Engine/EditorBlueprintResources/StandardMacros.Gate` false :!label _label_3
      (:`Exit`
        (bind _outhit (`KismetSystemLibrary.LineTraceSingleForObjects` _returnvalue (+ _returnvalue (* (`SceneComponent.GetForwardVector` _camera) (`self.fInteractionDistance`))) (`|MakeArray` "ObjectTypeQuery1" "ObjectTypeQuery2" "ObjectTypeQuery4" "ObjectTypeQuery7" :!type "EObjectTypeQuery Enum") false (`/Game/Blueprints/DesktopPawn/Inventory.Items` (`self.Inventory`)) "ForDuration" :!label _label_4))
        (bind (_bblockinghit _binitialoverlap _time _distance _location _impactpoint _normal _impactnormal _physmat _hitactor) (`GameplayStatics.BreakHitResult` _outhit))
        (if (and _bblockinghit (`KismetSystemLibrary.DoesImplementInterface` _hitactor "/Game/Blueprints/InteractionBPI.InteractionBPI_C"))
          (message `/Game/Blueprints/InteractionBPI.InteractWithObject` _hitactor self)))))
  (:`Released`
    (`/Engine/EditorBlueprintResources/StandardMacros.Gate` false :!label _label_5
      (:`Exit`
        (goto _label_4)))))

(event `Key|RightMouseButton`
  (params (Key :type "Key Structure"))
  (:`Pressed`
    (goto _label_5 :!via `Close`))
  (:`Released`
    (goto _label_5 :!via `Open`)))

(event `Key|RightMouseButton`
  (params (Key :type "Key Structure"))
  (:`Pressed`
    (goto _label_6 :!via `Close`))
  (:`Released`
    (goto _label_6 :!via `Open`)))

(event `InputAction|Drop`
  (params (Key :type "Key Structure"))
  (:`Pressed`
    (`/Engine/EditorBlueprintResources/StandardMacros.Gate` false :!label _label_6))
  (:`Released`
    (`/Engine/EditorBlueprintResources/StandardMacros.Gate` false :!label _label_7
      (:`Exit`
        (`/Game/Blueprints/DesktopPawn/Inventory.Drop Item` (`self.Inventory`) (`self.iCurrentInventorySlot`))))))

(event `Key|RightMouseButton`
  (params (Key :type "Key Structure"))
  (:`Pressed`
    (goto _label_7 :!via `Close`))
  (:`Released`
    (goto _label_7 :!via `Open`)))

(fn `Change Tools`
  (params (`New Tool Slot` :type Integer))
  (bind _icurrentinventoryslot (`self.iCurrentInventorySlot`))
  (if (!= `New Tool Slot` _icurrentinventoryslot)
    (`/Game/Blueprints/DesktopPawn/Inventory.Deselect Item` (`self.Inventory`) `New Tool Slot` _icurrentinventoryslot)
    (`/Game/Blueprints/DesktopPawn/Inventory.Select Item` (`self.Inventory`) `New Tool Slot`)
    (bind _output_get (set `self.iCurrentInventorySlot` `New Tool Slot`))
    (`KismetSystemLibrary.PrintString` (`KismetStringLibrary.Conv_IntToString` _output_get))))

(fn `Find Evidence`
  (returns (EvidenceHit :type "Array of Actor Object Reference") (EvidenceFound :type Boolean))
  (locals (fEvidenceFOV :type "Float (double-precision)" :default 7.5) (`Object World Types` :type "Array of EObjectTypeQuery Enum") (ViewedEvidence :type "Array of Actor Object Reference"))
  (bind _camera (`self.Camera`))
  (bind _viewedevidence (`local.ViewedEvidence`))
  (bind _returnvalue (`SceneComponent.K2_GetComponentLocation` _camera))
  ;[1 1 1] Sphere tracing extended 1.5 meters infront of the headset/player
  (bind _outhits (`KismetSystemLibrary.SphereTraceMultiForObjects` _returnvalue (+ _returnvalue (* (`SceneComponent.GetForwardVector` _camera) 150.0)) (`local.fEvidenceFOV`) (`local.Object World Types`)))
  (for _array_element _outhits
    ;[1 1 1] Create array of identified evidence
    (bind _asevidence (cast `/Game/Blueprints/Items/Evidence/Evidence` (`.HitActor` (`GameplayStatics.BreakHitResult` _array_element))))
    (`KismetArrayLibrary.Array_Add` _viewedevidence _asevidence))
  (return _viewedevidence (> (`KismetArrayLibrary.Array_Length` _viewedevidence) 0)))

(fn `Get Navmesh Pos`
  (params (`Initial Direction` :type "Vector Structure") (`Axis Value` :type "Float (double-precision)"))
  (returns (`Navmesh Position` :type "Vector Structure"))
  (return (`NavigationSystemV1.K2_ProjectPointToNavigation` (+ (* (* `Initial Direction` `Axis Value`) (`self.fCurrentMoveSpeed`)) (`self.vLastNavmeshPos`)))))

(fn `Navmesh To World Pos`
  (params (`Navmesh Position` :type "Vector Structure"))
  (returns (`World Position` :type "Vector Structure"))
  (bind _fcapsulehalfheight (`self.fCapsuleHalfHeight`))
  (bind _returnvalue (`CapsuleComponent.GetUnscaledCapsuleHalfHeight` (`self.Capsule`)))
  ;[1 1 1] Process Crouching Height Changes
  (if (not (== _returnvalue _fcapsulehalfheight))
    (`CapsuleComponent.SetCapsuleHalfHeight` (`self.Capsule`) (- _returnvalue (select `bool` (> _returnvalue _fcapsulehalfheight) :`false` -2.0 :`true` 2.0 :!type "Float (single-precision)")) true))
  (return (+ (`KismetMathLibrary.MakeVector` 0.0 0.0 (`CapsuleComponent.GetScaledCapsuleHalfHeight_WithoutHemisphere` (`self.Capsule`))) `Navmesh Position`)))

(fn `Pick Slot`
  (params (`Key Input` :type "Key Structure" :default "None") (Axis :type Integer))
  (returns (`New Tool Slot` :type Integer))
  (locals (aKeyPresses :type "Array of Key Structure") (iNumOfSlots :type Integer :default 9) (iNewSlot :type Integer) (AxisValue :type Integer))
  (bind _axisvalue (`local.AxisValue`))
  (bind _icurrentinventoryslot (`self.iCurrentInventorySlot`))
  (bind _output_get (set `local.AxisValue` Axis))
  (if (== _output_get 0)
    (set `local.iNewSlot` (`KismetArrayLibrary.Array_Find` (`local.aKeyPresses`) `Key Input`))
    (else
      ;[1 1 1] Scrollwheel
      (if (> _axisvalue 0)
        (if (== (`local.iNumOfSlots`) _icurrentinventoryslot)
          (set `local.iNewSlot` 0) ; Overflow to 0
          (else
            (set `local.iNewSlot` (+ (`self.iCurrentInventorySlot`) (`KismetMathLibrary.SignOfInteger` _axisvalue)) :!label _label) ; Add or Subtract 1
          ))
        (elif (== _icurrentinventoryslot 0)
          (set `local.iNewSlot` (`local.iNumOfSlots`)) ; Overflow to Max
          (else
            (goto _label))))))
  (return (`local.iNewSlot`)))

(fn `Pick Up Item`
  (params (Item :type "/Game/Blueprints/Items/Item Object Reference"))
  (bind _icurrentinventoryslot (`self.iCurrentInventorySlot`))
  (bind (_item _itemslot) (`/Game/Blueprints/DesktopPawn/Inventory.AddItemToInventory` (`self.Inventory`) Item _icurrentinventoryslot))
  (if (== _icurrentinventoryslot _itemslot)
    (`/Game/Blueprints/DesktopPawn/Inventory.Select Item` (`self.Inventory`) _icurrentinventoryslot)))

(fn `Spawn Tools`
  ;[1 1 1] Spawn tools
  (bind _asgame_mode_bp (cast `/Game/Blueprints/GameModeBP` (`GameplayStatics.GetGameMode`))
    (:`then`
      (set `/Game/Blueprints/DesktopPawn/Inventory.Owner` self (`self.Inventory`))
      (for (_array_element _array_index) (`/Game/Blueprints/GameModeBP.ToolTypes` _asgame_mode_bp)
        (bind _returnvalue (`|SpawnActorFromClass` _array_element (`self.GetTransform`) "AlwaysSpawn" "OverrideRootScale" null null))
        (`/Game/Blueprints/DesktopPawn/Inventory.AddItemToInventory` (`self.Inventory`) _returnvalue (+ _array_index 1))))
    (:`CastFailed`
      (`KismetSystemLibrary.QuitGame` null "Quit") ; Shouldn't Trigger
    )))

(fn `UserConstructionScript`
  (locals (ObjectTypes :type "Array of EObjectTypeQuery Enum") (CapsulePos :type "Transform Structure"))
  (bind _capsule (`self.Capsule`))
  (bind _capsule_2 (`self.Capsule`))
  (set `self.bUseControllerRotationYaw` true)
  (`self.K2_SetActorLocationAndRotation` (`SceneComponent.K2_GetComponentLocation` _capsule) (`SceneComponent.K2_GetComponentRotation` _capsule))
  ;[1 1 1] Teleports pawn above any objects overlapping capsule hitbox at the end of drag
  (`self.Do While` (stale _returnvalue)
    (:`Loop Body`
      (bind (_outactors _returnvalue) (`KismetSystemLibrary.ComponentOverlapActors` _capsule_2 (`SceneComponent.K2_GetComponentToWorld` _capsule_2) (`local.ObjectTypes`))) ; May have to add "Actors to Ignore" in future
      (if _returnvalue
        (`self.K2_AddActorWorldOffset` (0.0 0.0 1.0) false true)))))